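; BP_MyController is a player controller that aims the possessed cannon pawn from axis input.
; It caches the controlled pawn on BeginPlay.
; The horizontal axis adds controller yaw input to that pawn.
; The raise axis, when non-zero, casts the pawn to BP_Cannon and applies a scaled relative pitch rotation to its Arrow component, independent of control rotation.
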(event `InputAxis|LeftRigthCannon`
  (params (AxisValue :type "Float (single-precision)"))
  (`Pawn.AddControllerYawInput` (`self.PawnCannon`) AxisValue))

(event `InputAxis|RaiseCannon`
  (params (AxisValue :type "Float (single-precision)"))
  (if (!= AxisValue 0.0)
    (bind _asbp_cannon (cast `/Game/BP_Cannon` (`self.PawnCannon`)))
    (`SceneComponent.K2_AddRelativeRotation` (`/Game/BP_Cannon.Arrow` _asbp_cannon) (`KismetMathLibrary.MakeRotator` 0.0 (* AxisValue 5.0)) false false)))

(event `self.ReceiveBeginPlay`
  (set `self.PawnCannon` (`self.K2_GetPawn`)))

(fn `UserConstructionScript`)